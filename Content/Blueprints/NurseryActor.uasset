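; NurseryActor is a hoverable mesh prop with a text name label, configured per instance through mesh and name variables in the construction script.
; BeginPlay enables input, the mouse cursor and mouse-over events on the first player controller.
; Cursor enter and exit switch the mesh's custom depth, toggle the label's visibility, set the Trigger flag and call TriggerTrue or TriggerFalse accordingly.
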(event OnBeginCursorOver(StaticMesh)
  (params (TouchedComponent :type Primitive%20Component%20Object%20Reference))
  (Rendering|SetRenderCustomDepth (Variables|Default|GetStaticMesh) true)
  (Variables|Default|SetTrigger true)
  (if (Variables|Default|GetTrigger)
    (Rendering|ToggleVisibility (Variables|Default|GetNameRender) false)
    (Default|CallTriggerTrue)
    (else
      (Rendering|ToggleVisibility (Variables|Default|GetNameRender) false)
      (Default|CallTriggerFalse))))

(event OnEndCursorOver(StaticMesh)
  (params (TouchedComponent :type Primitive%20Component%20Object%20Reference))
  (Rendering|SetRenderCustomDepth (Variables|Default|GetStaticMesh) false)
  (Variables|Default|SetTrigger false)
  (if (Variables|Default|GetTrigger)
    (Rendering|ToggleVisibility (Variables|Default|GetNameRender) false)
    (Default|CallTriggerTrue)
    (else
      (Rendering|ToggleVisibility (Variables|Default|GetNameRender) false)
      (Default|CallTriggerFalse))))

(event EventBeginPlay
  (bind _returnvalue (Game|GetPlayerController 0))
  (Input|EnableInput _returnvalue)
  (Variables|/Script/Engine.PlayerController|SetbEnableMouseOverEvents _returnvalue true)
  (Variables|/Script/Engine.PlayerController|SetbShowMouseCursor _returnvalue true))

(fn ConstructionScript
  (Components|StaticMesh|SetStaticMesh (Variables|Default|GetStaticMesh) (Variables|Default|GetVariableMesh))
  (Rendering|Components|TextRender|SetText (Variables|Default|GetNameRender) (Utilities|Text|ToText(String) (Variables|Default|GetName))))
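; A baby character built from layered sprite planes, with a name text, that can wander the navmesh at a random walk speed set on BeginPlay.
; BabyMovement chains AI moves to random reachable points, retriggering on success or failure, but nothing here starts it.
; ChangeVariable stores passed-in traits and maps them to head, hair and eye materials; the face value is unused.
; Tick overrides rotation using only the camera look-at's roll.
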(event Custom|Event%20Baby%20Movement
  ;[1 1 1] Random Movement Function
  (if (not (Variables|Default|GetisMoving))
    (AI|AIMoveTo self (Class|NavigationSystem|GetRandomPointinNavigableRadius (Transformation|GetActorLocation) (Variables|Default|GetmoveRadius)) 0 5.0 false
      (:then
        (Variables|Default|SetisMoving true))
      (:OnSuccess
        (Variables|Default|SetisMoving false :!label _label)
        (CallFunction|EventBabyMovement))
      (:OnFail
        (goto _label)))))

(event EventBeginPlay
  ;[1 1 1] Calling RandomMovement Function
  (Utilities|FlowControl|Sequence
    (:then_0
      (bind _output_get (Variables|Default|SetmoveSpeed (Math|Random|RandomFloatinRange 1e+02 2e+02)))
      (Variables|/Script/Engine.CharacterMovementComponent|SetMaxWalkSpeed (Variables|Character|GetCharacterMovement) _output_get))))

(event EventTick
  (params (DeltaSeconds :type Float%20%28single-precision%29))
  ;[1 1 1] Face Rotation
  (Transformation|SetActorRotation (Math|Rotator|MakeRotator (- (.Roll (Math|Rotator|BreakRotator (Math|Rotator|FindLookatRotation (Transformation|GetActorLocation) (Camera|GetCameraLocation (Game|GetPlayerCameraManager 0))))) 9e+01) 0.0 0.0)))

(fn ConstructionScript)

(fn ChangeVariable
  (params (g_hairVar :type Float%20%28single-precision%29) (g_skinVar :type Float%20%28single-precision%29) (g_faceVar :type Float%20%28single-precision%29) (g_eyeVar :type Float%20%28single-precision%29) (g_name :type String))
  (bind _0_headplane (Variables|Default|Get0_headPlane))
  (bind _2_eyeplane (Variables|Default|Get2_eyePlane))
  (bind _1_hairplane (Variables|Default|Get1_hairPlane))
  (Variables|Default|SethairVar g_hairVar)
  (Variables|Default|SetskinVar g_skinVar)
  (Variables|Default|SetfaceVar g_faceVar)
  (Variables|Default|SeteyeVar g_eyeVar)
  (bind _output_get (Variables|Default|SetbabyName g_name))
  (Utilities|FlowControl|Sequence
    (:then_0
      ;[1 1 1] Change Head Sprite
      (if (== (Variables|Default|GetskinVar) 0.0)
        (Rendering|Material|SetMaterial _0_headplane 0 "/Game/Materials/UI/Baby/m_body1.m_body1")
        (elif (== (Variables|Default|GetskinVar) 1.0)
          (Rendering|Material|SetMaterial _0_headplane 0 "/Game/Materials/UI/Baby/m_body2.m_body2")
          (elif (== (Variables|Default|GetskinVar) 2.0)
            (Rendering|Material|SetMaterial _0_headplane 0 "/Game/Materials/UI/Baby/m_body3.m_body3")
            (elif (== (Variables|Default|GetskinVar) 3.0)
              (Rendering|Material|SetMaterial _0_headplane 0 "/Game/Materials/UI/Baby/m_body4.m_body4")
              (elif (== (Variables|Default|GetskinVar) 4.0)
                (Rendering|Material|SetMaterial _0_headplane 0 "/Game/Materials/UI/Baby/m_body5.m_body5")
                (elif (== (Variables|Default|GetskinVar) 5.0)
                  (Rendering|Material|SetMaterial _0_headplane 0 "/Game/Materials/UI/Baby/m_body6.m_body6"))))))))
    (:then_1
      ;[1 1 1] Change Hair Sprite
      (if (== (Variables|Default|GethairVar) 0.0)
        (Rendering|Material|SetMaterial _1_hairplane 0 "/Game/Materials/UI/Baby/m_babyHair1.m_babyHair1")
        (elif (== (Variables|Default|GethairVar) 1.0)
          (Rendering|Material|SetMaterial _1_hairplane 0 "/Game/Materials/UI/Baby/m_babyHair2.m_babyHair2")
          (elif (== (Variables|Default|GethairVar) 2.0)
            (Rendering|Material|SetMaterial _1_hairplane 0 "/Game/Materials/UI/Baby/m_babyHair3.m_babyHair3")
            (elif (== (Variables|Default|GethairVar) 3.0)
              (Rendering|Material|SetMaterial _1_hairplane 0 "/Game/Materials/UI/Baby/m_babyHair4.m_babyHair4")
              (elif (== (Variables|Default|GethairVar) 4.0)
                (Rendering|Material|SetMaterial _1_hairplane 0 "/Game/Materials/UI/Baby/m_babyHair5.m_babyHair5")
                (elif (== (Variables|Default|GethairVar) 5.0)
                  (Rendering|Material|SetMaterial _1_hairplane 0 "/Game/Materials/UI/Baby/m_babyHair6.m_babyHair6"))))))))
    (:then_2
      ;[1 1 1] Change Eye Sprite
      (if (== (Variables|Default|GeteyeVar) 0.0)
        (Rendering|Material|SetMaterial _2_eyeplane 0 "/Game/Materials/UI/Baby/m_eyes1.m_eyes1")
        (elif (== (Variables|Default|GeteyeVar) 1.0)
          (Rendering|Material|SetMaterial _2_eyeplane 0 "/Game/Materials/UI/Baby/m_eyes2.m_eyes2")
          (elif (== (Variables|Default|GeteyeVar) 2.0)
            (Rendering|Material|SetMaterial _2_eyeplane 0 "/Game/Materials/UI/Baby/m_eyes3.m_eyes3")
            (elif (== (Variables|Default|GeteyeVar) 3.0)
              (Rendering|Material|SetMaterial _2_eyeplane 0 "/Game/Materials/UI/Baby/m_eyes3.m_eyes3")
              (elif (== (Variables|Default|GeteyeVar) 4.0)
                (Rendering|Material|SetMaterial _2_eyeplane 0 "/Game/Materials/UI/Baby/m_eyes4.m_eyes4")
                (elif (== (Variables|Default|GeteyeVar) 5.0)
                  (Rendering|Material|SetMaterial _2_eyeplane 0 "/Game/Materials/UI/Baby/m_eyes5.m_eyes5"))))))))
    (:then_3
      (Rendering|Components|TextRender|SetText (Variables|Default|GetnameText) (Utilities|Text|ToText(String) _output_get)))))
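; randomCharacter is a wandering AI character that roams the navmesh at its own random pace.
; BeginPlay picks a random walk speed and applies it to CharacterMovement.
; Tick uses an IsWalking flag to issue one AIMoveTo at a time, toward a random navigable point within WalkRadius of its current location.
; Success or failure clears the flag, so the next Tick starts another move.
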(event EventBeginPlay
  (bind _output_get (Variables|Default|SetWalkSpeed (Math|Random|RandomFloatinRange 1e+02 6e+02)))
  (Variables|/Script/Engine.CharacterMovementComponent|SetMaxWalkSpeed (Variables|Character|GetCharacterMovement) _output_get))

(event EventTick
  (params (DeltaSeconds :type Float%20%28single-precision%29))
  (if (not (Variables|Default|GetIsWalking))
    (AI|AIMoveTo self (Class|NavigationSystem|GetRandomPointinNavigableRadius (Transformation|GetActorLocation) (Variables|Default|GetWalkRadius)) 0 5.0 false
      (:then
        (Variables|Default|SetIsWalking true))
      (:OnSuccess
        (Variables|Default|SetIsWalking false :!label _label))
      (:OnFail
        (goto _label)))))

(fn ConstructionScript)
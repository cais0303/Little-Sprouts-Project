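; Clickable hazard object actor that shows an information menu with its name and description.
; The first click creates a MenuTemplate widget, passes in the object's name and description and adds it to the viewport; later clicks make the cached widget visible again.
; Cursor hover toggles custom depth rendering on the static mesh.
; The construction script assigns the mesh from a variable, allowing different meshes per instance.
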(event OnClicked(staticMesh)
  (params (TouchedComponent :type Primitive%20Component%20Object%20Reference) (ButtonPressed :type Key%20Structure :default "AnyKey"))
  (if (Variables|Default|GethasWidget)
    (Widget|SetVisibility (Variables|Default|GetwidgetReference) "Visible")
    (else
      (bind _returnvalue (UserInterface|CreateWidget "/Game/UI/MenuTemplate.MenuTemplate_C" (Game|GetPlayerController 0)))
      (bind _output_get (Variables|Default|SetwidgetReference _returnvalue))
      (Variables|/Game/UI/MenuTemplate.MenuTemplate_C|SetobjName _output_get (Variables|Default|GetobjectName))
      (Variables|/Game/UI/MenuTemplate.MenuTemplate_C|SetobjDesc _output_get (Variables|Default|GetobjectDescription))
      (UserInterface|Viewport|AddtoViewport _returnvalue 0)
      (Variables|Default|SethasWidget true))))

(event OnEndCursorOver(staticMesh)
  (params (TouchedComponent :type Primitive%20Component%20Object%20Reference))
  (Rendering|SetRenderCustomDepth (Variables|Mesh|GetStaticMesh) false))

(event OnBeginCursorOver(staticMesh)
  (params (TouchedComponent :type Primitive%20Component%20Object%20Reference))
  (Rendering|SetRenderCustomDepth (Variables|Mesh|GetStaticMesh) true))

(fn ConstructionScript
  (Components|StaticMesh|SetStaticMesh (Variables|Default|GetstaticMesh) (Variables|Default|GetvariableMesh)))
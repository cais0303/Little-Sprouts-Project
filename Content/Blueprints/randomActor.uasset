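; An interactive actor that highlights on mouse hover or actor overlap and broadcasts its trigger state.
; BeginPlay enables input, the cursor and mouse-over events, and creates a dynamic material instance from M_ChangeColor.
; Cursor and overlap events share paths that switch the mesh between blue and green and set the Trigger flag.
; Each change toggles the Name component's visibility and calls TriggerTrue or TriggerFalse to match the flag.
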(event OnBeginCursorOver(StaticMesh)
  (params (TouchedComponent :type Primitive%20Component%20Object%20Reference))
  (Rendering|Material|SetVectorParameterValue (stale EventBeginPlay _returnvalue_2) "Color" "(R=0.000000,G=0.422478,B=1.000000,A=1.000000)" :!class /Script/Engine.MaterialInstanceDynamic)
  (Variables|Default|SetTrigger true)
  (if (Variables|Default|GetTrigger)
    (Rendering|ToggleVisibility (Variables|Default|GetName) false)
    (Default|CallTriggerTrue)
    (else
      (Rendering|ToggleVisibility (Variables|Default|GetName) false)
      (Default|CallTriggerFalse))))

(event OnEndCursorOver(StaticMesh)
  (params (TouchedComponent :type Primitive%20Component%20Object%20Reference))
  (Rendering|Material|SetVectorParameterValue (stale EventBeginPlay _returnvalue_2) "Color" "(R=0.217231,G=1.000000,B=0.000000,A=1.000000)" :!class /Script/Engine.MaterialInstanceDynamic)
  (Variables|Default|SetTrigger false)
  (if (Variables|Default|GetTrigger)
    (Rendering|ToggleVisibility (Variables|Default|GetName) false)
    (Default|CallTriggerTrue)
    (else
      (Rendering|ToggleVisibility (Variables|Default|GetName) false)
      (Default|CallTriggerFalse))))

(event EventBeginPlay
  (bind _returnvalue (Game|GetPlayerController 0))
  (Input|EnableInput _returnvalue)
  (Variables|/Script/Engine.PlayerController|SetbEnableMouseOverEvents _returnvalue true)
  (Variables|/Script/Engine.PlayerController|SetbShowMouseCursor _returnvalue true)
  (bind _returnvalue_2 (Rendering|Material|CreateDynamicMaterialInstance (Variables|Default|GetStaticMesh) 0 "/Game/Materials/M_ChangeColor.M_ChangeColor" :!class /Script/Engine.PrimitiveComponent)))

(event Collision|EventActorBeginOverlap
  (params (OtherActor :type Actor%20Object%20Reference))
  (Rendering|Material|SetVectorParameterValue (stale EventBeginPlay _returnvalue_2) "Color" "(R=0.000000,G=0.422478,B=1.000000,A=1.000000)" :!class /Script/Engine.MaterialInstanceDynamic)
  (Variables|Default|SetTrigger true)
  (if (Variables|Default|GetTrigger)
    (Rendering|ToggleVisibility (Variables|Default|GetName) false)
    (Default|CallTriggerTrue)
    (else
      (Rendering|ToggleVisibility (Variables|Default|GetName) false)
      (Default|CallTriggerFalse))))

(event Collision|EventActorEndOverlap
  (params (OtherActor :type Actor%20Object%20Reference))
  (Rendering|Material|SetVectorParameterValue (stale EventBeginPlay _returnvalue_2) "Color" "(R=0.217231,G=1.000000,B=0.000000,A=1.000000)" :!class /Script/Engine.MaterialInstanceDynamic)
  (Variables|Default|SetTrigger false)
  (if (Variables|Default|GetTrigger)
    (Rendering|ToggleVisibility (Variables|Default|GetName) false)
    (Default|CallTriggerTrue)
    (else
      (Rendering|ToggleVisibility (Variables|Default|GetName) false)
      (Default|CallTriggerFalse))))

(fn ConstructionScript)